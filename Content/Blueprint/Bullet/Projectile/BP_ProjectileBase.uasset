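; BP_ProjectileBase is a base projectile that applies Gameplay Ability System effects to what it hits.
; The construction script copies its speed, gravity scale and rotation-follows-velocity variables into the projectile movement component.
; On a collision hit, it applies each effect class in the OnHitGameplayEffect map, using the mapped value as magnitude, if the other actor has an ability system component.
; It prints an error for null classes and destroys itself after any hit.
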(event `self.Collision.OnComponentHit`
  (params (HitComponent :type "PrimitiveComponent Object Reference") (OtherActor :type "Actor Object Reference") (OtherComp :type "PrimitiveComponent Object Reference") (NormalImpulse :type "Vector Structure") (Hit :type "HitResult Structure (by ref)"))
  (bind _returnvalue (`AbilitySystemBlueprintLibrary.GetAbilitySystemComponent` OtherActor))
  (bind _onhitgameplayeffect (`self.OnHitGameplayEffect`))
  ;[1 0.03955 0.03955] On Hit Apply Gameplay Effects
  (`/Engine/EditorBlueprintResources/StandardMacros.IsValid` _returnvalue
    (:`Is Valid`
      (bind _keys (`BlueprintMapLibrary.Map_Keys` _onhitgameplayeffect))
      (for _array_element _keys
        (if (`KismetSystemLibrary.IsValidClass` _array_element)
          (`self.ApplyEffectToAbilitySystemComponent` _returnvalue _array_element (`BlueprintMapLibrary.Map_Find` _onhitgameplayeffect _array_element))
          (else
            (`KismetSystemLibrary.PrintString` "ProjectileBase: Null class in projectile object" true true (struct :`R` 1.0 :`G` 0.039546 :`B` 0.039546 :`A` 1.0) 5.0)))))
    (:`Is Not Valid`
      _))
  (`self.K2_DestroyActor`))

(fn `UserConstructionScript`
  (bind _projectilemovementcomponent (`self.ProjectileMovementComponent`))
  (set `ProjectileMovementComponent.InitialSpeed` (`self.InitialMovementSpeed`) _projectilemovementcomponent)
  (set `ProjectileMovementComponent.MaxSpeed` (`self.MaxMovementSpeed`) _projectilemovementcomponent)
  (set `ProjectileMovementComponent.ProjectileGravityScale` (`self.GravityScale`) _projectilemovementcomponent)
  (set `ProjectileMovementComponent.bRotationFollowsVelocity` (`self.RotationFollowsVelocity`) _projectilemovementcomponent))