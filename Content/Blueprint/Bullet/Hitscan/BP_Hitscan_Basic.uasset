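; BP_Hitscan_Basic is a basic hitscan bullet that applies gameplay effects to what it hits.
; On a blocking hit, it applies each effect class in the OnHitGameplayEffect map, with its mapped magnitude, to the hit actor's Ability System Component.
; It then spawns Niagara impact dust along the surface normal and destroys itself.
; The trace is not in this graph; the hit arrives through the ApplyGameplayEffectstoHit event.
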(event `self.ApplyGameplayEffectsToHit`
  (params (Hit :type "HitResult Structure"))
  (bind (_bblockinghit _binitialoverlap _time _distance _location _impactpoint _normal _impactnormal _physmat _hitactor) (`GameplayStatics.BreakHitResult` Hit))
  (bind (_bblockinghit_2 _binitialoverlap_2 _time_2 _distance_2 _location_2 _impactpoint_2 _normal_2) (`GameplayStatics.BreakHitResult` Hit))
  (bind _onhitgameplayeffect (`self.OnHitGameplayEffect`))
  (bind _returnvalue (`AbilitySystemBlueprintLibrary.GetAbilitySystemComponent` _hitactor))
  (if _bblockinghit
    (`/Engine/EditorBlueprintResources/StandardMacros.IsValid` _returnvalue
      (:`Is Valid`
        (bind _keys (`BlueprintMapLibrary.Map_Keys` _onhitgameplayeffect))
        (for _array_element _keys
          (if (`KismetSystemLibrary.IsValidClass` _array_element)
            (`self.ApplyEffectToAbilitySystemComponent` _returnvalue _array_element (`BlueprintMapLibrary.Map_Find` _onhitgameplayeffect _array_element) Hit)
            (else
              (`KismetSystemLibrary.PrintString` "ProjectileBase: Null class in projectile object" true true (struct :`R` 1.0 :`G` 0.039546 :`B` 0.039546 :`A` 1.0) 5.0)))))
      (:`Is Not Valid`
        _))
    (`NiagaraFunctionLibrary.SpawnSystemAtLocation` "/Game/VFX/NS_ImpactDust.NS_ImpactDust" _location_2 (`KismetMathLibrary.MakeRotFromX` _normal_2))
    (`self.K2_DestroyActor`)))

(fn `UserConstructionScript`
  (`parent.UserConstructionScript`))