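; GA_AirDash is a Gameplay Ability that dashes the owning actor along its movement input.
; On activation it commits, reads a float attribute from the Ability System Component as dash strength, and gets input direction and movement component through messages to the owner.
; If the attribute is found, it applies their product as a velocity-change impulse.
; The ability ends immediately and contains no airborne check of its own.
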(event `self.K2_ActivateAbility`
  (bind (_owneractor _avataractor _playercontroller _abilitysystemcomponent) (break `GameplayAbilityActorInfo` (`self.GetActorInfo`)))
  (bind (_bsuccessfullyfoundattribute _returnvalue) (`AbilitySystemBlueprintLibrary.GetFloatAttributeFromAbilitySystemComponent` _abilitysystemcomponent (struct :`AttributeName` "AirDashSpeed" :`Attribute` "/Script/Collab09FPS.DashAttributeSet:AirDashSpeed" :`AttributeOwner` "/Script/CoreUObject.Class'/Script/Collab09FPS.DashAttributeSet'")))
  (bind _returnvalue_2 (`self.K2_CommitAbility`))
  (if _returnvalue_2
    (bind _returnvalue_3 (message `CharacterMovementAbilities.GetMovementInput` _owneractor))
    (if _bsuccessfullyfoundattribute
      (bind _returnvalue_4 (message `CharacterMovementAbilities.ActorCharacterMovementComponent` _owneractor))
      (`CharacterMovementComponent.AddImpulse` _returnvalue_4 (* _returnvalue_3 _returnvalue) true))
    (`self.K2_EndAbility`)
    (else
      (`self.K2_EndAbility`))))