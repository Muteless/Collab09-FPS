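; Gameplay ability, activated by a gameplay event, that opens and closes the elemental wheel for a player-controlled character.
; After committing, it messages the player controller to open the weapon wheel, shows the cursor centered in the viewport and enables game-and-UI input.
; It waits for the ElementalWheel Close event, then closes the wheel, restores game-only input and ends.
; A failed commit ends it immediately, as does a missing controller after printing an error.
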(event `self.K2_ActivateAbilityFromEvent`
  (params (EventData :type "GameplayEventData Structure (by ref)"))
  (bind (_owneractor _avataractor _playercontroller) (break `GameplayAbilityActorInfo` (`self.GetActorInfo`)))
  (bind (_owneractor_2 _avataractor_2 _playercontroller_2) (break `GameplayAbilityActorInfo` (`self.GetActorInfo`)))
  (bind (_x _y) (`KismetMathLibrary.BreakVector2D` (/ (`WidgetLayoutLibrary.GetViewportSize`) (2.0 2.0))))
  (`|SwitchGameplayTag` (`.EventTag` (break `GameplayEventData` EventData))
    (:`Event.Ability.ElementalWheel.Open`
      (bind _returnvalue (`self.K2_CommitAbility`))
      (if _returnvalue
        (`/Engine/EditorBlueprintResources/StandardMacros.IsValid` _playercontroller_2
          (:`Is Valid`
            (message `CharacterController.OpenWeaponWheel` _playercontroller_2)
            (set `PlayerController.bShowMouseCursor` true _playercontroller_2)
            (`WidgetBlueprintLibrary.SetInputMode_GameAndUIEx` _playercontroller_2 null)
            (`PlayerController.SetMouseLocation` _playercontroller_2 (`KismetMathLibrary.FTrunc` _x) (`KismetMathLibrary.FTrunc` _y))
            (bind _asynctaskproxy (`AbilityTask_WaitGameplayEvent.WaitGameplayEvent` (struct :`TagName` "Event.Ability.ElementalWheel.Close") null)
              (:`EventReceived`
                (message `CharacterController.CloseWeaponWheel` _playercontroller)
                (set `PlayerController.bShowMouseCursor` false _playercontroller)
                (`WidgetBlueprintLibrary.SetInputMode_GameOnly` _playercontroller)
                (`GameplayTask.EndTask` _asynctaskproxy)
                (`self.K2_EndAbility`))))
          (:`Is Not Valid`
            (`KismetSystemLibrary.PrintString` "ERROR: ElementalWheel called from non player controller character!" true true (struct :`R` 1.0 :`G` 0.057804 :`A` 1.0))
            (`self.K2_EndAbility`)))
        (else
          (`self.K2_EndAbility`))))))