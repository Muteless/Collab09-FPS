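; GA_WallRun is a Gameplay Ability that starts and ends wall running for its owner.
; After committing, it switches on the triggering event tag: the wall run tag messages the owner to begin movement, while the end tag ends the ability.
; Once running, it waits for a WallRunEnd gameplay event to end itself, and a failed commit ends it immediately.
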(event `self.K2_ActivateAbility`
  (bind _returnvalue (`self.K2_CommitAbility` :!label _label))
  (if _returnvalue
    (`|SwitchGameplayTag` (`.EventTag` (break `GameplayEventData` (`self.CurrentEventData`)))
      (:`Event.Ability.WallRun`
        (message `CharacterMovementAbilities.CharacterMovementWallRun` (`.OwnerActor` (break `GameplayAbilityActorInfo` (`self.GetActorInfo`))))
        (`AbilityTask_WaitGameplayEvent.WaitGameplayEvent` (struct :`TagName` "Event.Ability.WallRunEnd") null
          (:`EventReceived`
            (`self.K2_EndAbility`))))
      (:`Event.Ability.WallRunEnd`
        (`self.K2_EndAbility`)))
    (else
      (`self.K2_EndAbility`))))

(event `self.K2_ActivateAbilityFromEvent`
  (params (EventData :type "GameplayEventData Structure (by ref)"))
  (goto _label))