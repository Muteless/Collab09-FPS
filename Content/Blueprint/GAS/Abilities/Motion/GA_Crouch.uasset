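; GA_Crouch is an event-triggered Gameplay Ability that crouches and uncrouches its owner, or starts a slide when the owner moves fast enough.
; On the crouch event it compares owner velocity against a float attribute, either granting and activating GA_Sliding once with a slide event, or committing and sending a crouch message.
; The uncrouch event and ability end both send an uncrouch message to the owner.
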(event `self.K2_ActivateAbilityFromEvent`
  (params (EventData :type "GameplayEventData Structure (by ref)"))
  (bind (_owneractor _avataractor _playercontroller _abilitysystemcomponent) (break `GameplayAbilityActorInfo` (`self.GetActorInfo`)))
  (bind (_bsuccessfullyfoundattribute _returnvalue) (`AbilitySystemBlueprintLibrary.GetFloatAttributeFromAbilitySystemComponent` _abilitysystemcomponent (struct :`AttributeName` "SlidingMinSpeed" :`Attribute` "/Script/Collab09FPS.CMCAttributeSet:SlidingMinSpeed" :`AttributeOwner` "/Script/CoreUObject.Class'/Script/Collab09FPS.CMCAttributeSet'")))
  ;[1 0.03955 0.03955] Start
  (`|SwitchGameplayTag` (`.EventTag` (break `GameplayEventData` EventData))
    (:`Event.Ability.Crouch`
      (if _bsuccessfullyfoundattribute
        (if (>= (`KismetMathLibrary.VSize` (`Actor.GetVelocity` _owneractor)) _returnvalue)
          (`AbilitySystemComponent.K2_GiveAbilityAndActivateOnce` (`.AbilitySystemComponent` (break `GameplayAbilityActorInfo` (`self.GetActorInfo`))) "/Game/Blueprint/GAS/Abilities/Motion/GA_Sliding.GA_Sliding_C" 0 -1)
          (`self.SendGameplayEvent` (struct :`TagName` "Event.Ability.Slide"))
          (else
            (bind _returnvalue_2 (`self.K2_CommitAbility`))
            (if _returnvalue_2
              ;[0 0.3916 0.8879] Crouch
              (message `CharacterMovementAbilities.CharacterMovementCrouch` (`.OwnerActor` (break `GameplayAbilityActorInfo` (`self.GetActorInfo`))))
              (else
                (`self.K2_EndAbility`)))))
        (else
          (`self.K2_EndAbility`))))
    (:`Event.Ability.UnCrouch`
      (message `CharacterMovementAbilities.CharacterMovementUncrouch` (`.OwnerActor` (break `GameplayAbilityActorInfo` (`self.GetActorInfo`))) :!label _label)
      (`self.K2_EndAbility`))))

(event `self.K2_OnEndAbility`
  (params (bWasCancelled :type Boolean))
  (goto _label))