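; GA_WallRun is a Gameplay Ability that runs the character's wall-run state, driven by gameplay event tags.
; On a Wall Run event it commits, sends a wall-run message to the owner, and applies GE_WallRunning to itself.
; It then waits for a WallRunEnd event to end, while a failed commit or end-tag activation ends it immediately.
; Ending the ability removes the effect by its stored handle.
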(event `self.K2_ActivateAbilityFromEvent`
  (params (EventData :type "GameplayEventData Structure (by ref)"))
  (bind (_owneractor _avataractor _playercontroller _abilitysystemcomponent) (break `GameplayAbilityActorInfo` (`self.GetActorInfo`)))
  (`|SwitchGameplayTag` (`.EventTag` (break `GameplayEventData` (`self.CurrentEventData`))) :!label _label
    (:`Event.Ability.WallRun`
      (bind _returnvalue (`self.K2_CommitAbility`))
      (if _returnvalue
        (message `CharacterMovementAbilities.CharacterMovementWallRun` (`.OwnerActor` (break `GameplayAbilityActorInfo` (`self.GetActorInfo`))))
        (bind _returnvalue_2 (`AbilitySystemComponent.BP_ApplyGameplayEffectToSelf` _abilitysystemcomponent "/Game/Blueprint/GAS/Effects/Movement/GE_WallRunning.GE_WallRunning_C" 0.0 (`AbilitySystemComponent.MakeEffectContext` _abilitysystemcomponent)))
        (set `self.WallRunEffect` _returnvalue_2)
        (bind _asynctaskproxy (`AbilityTask_WaitGameplayEvent.WaitGameplayEvent` (struct :`TagName` "Event.Ability.WallRunEnd") null true)
          (:`EventReceived`
            (set `self.Async Task` _asynctaskproxy)
            (`self.K2_EndAbility`)))
        (else
          (`self.K2_EndAbility` :!label _label_2))))
    (:`Event.Ability.WallRunEnd`
      (goto _label_2))))

(event `self.K2_ActivateAbility`
  (goto _label))

(event `self.K2_OnEndAbility`
  (params (bWasCancelled :type Boolean))
  (bind _async_task (`self.Async Task`))
  (`/Engine/EditorBlueprintResources/StandardMacros.IsValid` _async_task
    (:`Is Valid`
      (`GameplayTask.EndTask` _async_task))
    (:`Is Not Valid`
      _))
  (`self.BP_RemoveGameplayEffectFromOwnerWithHandle` (`self.WallRunEffect`)))