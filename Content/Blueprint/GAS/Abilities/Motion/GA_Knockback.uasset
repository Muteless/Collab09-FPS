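; GA_Knockback is a Gameplay Ability that sets up a knockback on its avatar from gameplay event data.
; On activation it reads the first hit result in the target data, using its Distance field as Strength.
; Direction is the hit Normal plus the avatar's reversed forward vector, left unnormalized.
; It then hands off to the parent class's activation, with no end-of-ability logic of its own.
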(event `self.K2_ActivateAbility`
  (bind (_bblockinghit _binitialoverlap _time _distance _location _impactpoint _normal) (`GameplayStatics.BreakHitResult` (`AbilitySystemBlueprintLibrary.GetHitResultFromTargetData` (`.TargetData` (break `GameplayEventData` (`self.CurrentEventData`))))))
  (set `self.Strength` _distance)
  (set `self.Direction` (+ _normal (* (`Actor.GetActorForwardVector` (`self.GetAvatarActorFromActorInfo`)) -1.0)))
  (`parent.K2_ActivateAbility`))