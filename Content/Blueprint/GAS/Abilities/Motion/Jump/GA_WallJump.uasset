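; GA_WallJump is a Gameplay Ability that ends the owner's wall run and launches a jump.
; On a successful commit, it reads a strength value from an ability system attribute and, if found, sends end-wall-run and jump messages to the owner's movement.
; The jump resets Z velocity, with direction from the component-wise product of actor up and forward vectors.
; The ability ends immediately afterward; a debug "Hello" print remains on activation.
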(event `self.K2_ActivateAbility`
  (bind (_owneractor _avataractor _playercontroller _abilitysystemcomponent) (break `GameplayAbilityActorInfo` (`self.GetActorInfo`)))
  (bind (_bfound _returnvalue) (`AbilitySystemComponent.GetGameplayAttributeValue` _abilitysystemcomponent (struct :`AttributeName` "WallJumpZVelocity" :`Attribute` "/Script/Collab09FPS.CMCAttributeSet:WallJumpZVelocity" :`AttributeOwner` "/Script/CoreUObject.Class'/Script/Collab09FPS.CMCAttributeSet'")))
  (`KismetSystemLibrary.PrintString` "Hello")
  (bind _returnvalue_2 (`self.K2_CommitAbility`))
  (if _returnvalue_2
    (if _bfound
      (message `CharacterMovementAbilities.CharacterMovementEndWallRun` _owneractor)
      (message `CharacterMovementAbilities.CharacterMovementJump` _owneractor (* (`Actor.GetActorUpVector` _owneractor) (`Actor.GetActorForwardVector` _owneractor)) _returnvalue true)))
  (`self.K2_EndAbility`))