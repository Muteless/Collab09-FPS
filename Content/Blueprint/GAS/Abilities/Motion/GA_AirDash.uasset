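; GA_AirDash is a Gameplay Ability that dashes the owning character along its movement input.
; It ends without committing when input magnitude is below 0.3, and otherwise commits before acting.
; A float attribute from the Ability System Component scales the input into a velocity-change impulse on the movement component.
; Vertical velocity is then zeroed, and the ability ends immediately.
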(event `self.K2_ActivateAbility`
  (bind (_owneractor _avataractor _playercontroller _abilitysystemcomponent) (break `GameplayAbilityActorInfo` (`self.GetActorInfo`)))
  (bind (_bsuccessfullyfoundattribute _returnvalue) (`AbilitySystemBlueprintLibrary.GetFloatAttributeFromAbilitySystemComponent` _abilitysystemcomponent (struct :`AttributeName` "AirDashSpeed" :`Attribute` "/Script/Collab09FPS.DashAttributeSet:AirDashSpeed" :`AttributeOwner` "/Script/CoreUObject.Class'/Script/Collab09FPS.DashAttributeSet'")))
  (bind _returnvalue_2 (message `CharacterMovementAbilities.GetMovementInput` (`.OwnerActor` (break `GameplayAbilityActorInfo` (`self.GetActorInfo`)))))
  (if (not (< (`KismetMathLibrary.VSize` _returnvalue_2) 0.3))
    (bind _returnvalue_3 (`self.K2_CommitAbility`))
    (if _returnvalue_3
      (bind _returnvalue_4 (message `CharacterMovementAbilities.GetMovementInput` _owneractor))
      (if _bsuccessfullyfoundattribute
        (bind _returnvalue_5 (message `CharacterMovementAbilities.GetActorCharacterMovementComponent` _owneractor))
        (`CharacterMovementComponent.AddImpulse` _returnvalue_5 (* _returnvalue_4 _returnvalue) true)
        (bind (_velocity_x _velocity_y) (`KismetMathLibrary.BreakVector` (`MovementComponent.Velocity` _returnvalue_5)))
        (set `MovementComponent.Velocity` (`KismetMathLibrary.MakeVector` _velocity_x _velocity_y) _returnvalue_5))
      (`self.K2_EndAbility`)
      (else
        (`self.K2_EndAbility`)))
    (else
      (`self.K2_EndAbility`))))