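; Gameplay Ability that handles the owning actor's slide movement, activated by a gameplay event.
; On a successful commit it messages the owner to start sliding, then waits once for the Event.Ability.StopSlide gameplay event.
; That event messages the owner to stop sliding and ends the ability, while a failed commit ends it immediately.
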(event `self.K2_ActivateAbilityFromEvent`
  (params (EventData :type "GameplayEventData Structure (by ref)"))
  (bind _owneractor (break `GameplayAbilityActorInfo` (`self.GetActorInfo`)))
  (`|SwitchGameplayTag` (`.EventTag` (break `GameplayEventData` EventData))
    (:`Event.Ability.StartSlide`
      (bind _returnvalue (`self.K2_CommitAbility`))
      (if _returnvalue
        (message `CharacterMovementAbilities.CharacterMovementStartSliding` _owneractor)
        (`AbilityTask_WaitGameplayEvent.WaitGameplayEvent` (struct :`TagName` "Event.Ability.StopSlide") null true
          (:`EventReceived`
            (message `CharacterMovementAbilities.CharacterMovementStopSliding` _owneractor)
            (`self.K2_EndAbility`)))
        (else
          (`self.K2_EndAbility`))))))

(event `self.K2_OnEndAbility`
  (params (bWasCancelled :type Boolean)))