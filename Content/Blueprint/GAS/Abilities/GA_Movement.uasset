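; GA_Movement is a Gameplay Ability that sends a move request to the owning actor.
; On activation it commits the ability, reads the hit location from the first target data entry of the triggering event, and passes it to the owner via a CharacterMovementMoveMessage call.
; The ability ends immediately afterward, or straight away if the commit fails.
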(event `self.K2_ActivateAbility`
  (bind _returnvalue (`self.K2_CommitAbility`))
  (if _returnvalue
    (message `CharacterMovementAbilities.CharacterMovementMove` (`.OwnerActor` (break `GameplayAbilityActorInfo` (`self.GetActorInfo`))) (`.Location` (`GameplayStatics.BreakHitResult` (`AbilitySystemBlueprintLibrary.GetHitResultFromTargetData` (`.TargetData` (break `GameplayEventData` (`self.CurrentEventData`)))))))
    (`self.K2_EndAbility`)
    (else
      (`self.K2_EndAbility`))))