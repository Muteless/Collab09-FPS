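; BP_TransitionLevel is a level-exit portal that unlocks once enough spawners have finished.
; It hides its Niagara effects on BeginPlay, and each EnablePortal call counts one finished spawner until the total is reached, then shows the effects and enables the portal.
; Overlapping the box while enabled reads the world index from the Game Instance and requests a transition to the next index through message calls.
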(event `self.ReceiveBeginPlay`
  (for _array_element (`self.NS`)
    (`/Engine/EditorBlueprintResources/StandardMacros.IsValid` _array_element
      (:`Is Valid`
        (`SceneComponent.SetVisibility` (`NiagaraActor.NiagaraComponent` _array_element) false false)))))

(event `self.Box.OnComponentBeginOverlap`
  (params (OverlappedComponent :type "PrimitiveComponent Object Reference") (OtherActor :type "Actor Object Reference") (OtherComp :type "PrimitiveComponent Object Reference") (OtherBodyIndex :type Integer) (bFromSweep :type Boolean) (SweepResult :type "HitResult Structure (by ref)"))
  (bind _returnvalue (`GameplayStatics.GetGameInstance`))
  (if (`self.Enabled?`)
    (bind _returnvalue_2 (message `GameInstanceInterface.GetWorldIndex` _returnvalue))
    (message `GameInstanceInterface.TransitionLevel` _returnvalue (+ _returnvalue_2 1))))

(event `IPortalEnableInterface.EnablePortal`
  (bind _result (`/Engine/EditorBlueprintResources/StandardMacros.IncrementInt` (`self.CurrentFinishedSpawners`))
    (:`  `
      (if (>= _result (`self.TotalSpawners`))
        (for _array_element (`self.NS`)
          (`SceneComponent.SetVisibility` (`NiagaraActor.NiagaraComponent` _array_element) true false)
          (set `self.Enabled?` true))))))

(fn `UserConstructionScript`)