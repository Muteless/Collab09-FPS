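; BP_PlayerCharacter is the player character Blueprint, handling movement input.
; The IAMove input event checks that the AbilitySystemComponent has all tags in MovementTag, so gameplay tags gate movement.
; While triggered, it feeds the input's X and Y into AddMovementInput along the capsule's right and forward vectors, so movement follows capsule orientation.
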(event `/Game/Blueprint/Interface/BPI_Input.IA_Move`
  (params (InputType :type "/Game/Enumeration/E_InputType Enum" :default "NewEnumerator0") (Input :type "Vector2D Structure"))
  (bind (_x _y) (`KismetMathLibrary.BreakVector2D` Input))
  ;[0.2502 0 0] Movement
  ;[1 1 1] Check Movement Requirements
  (if (`GameplayTagAssetInterface.HasAllMatchingGameplayTags` (`self.AbilitySystemComponent`) (`self.MovementTag`))
    ;[0 0.3916 0.8879] Produce Movement
    (switch `/Game/Enumeration/E_InputType` InputType
      (:`NewEnumerator1`
        (`self.AddMovementInput` (`SceneComponent.GetRightVector` (`self.CapsuleComponent`)) _x)
        (`self.AddMovementInput` (`SceneComponent.GetForwardVector` (`self.CapsuleComponent`)) _y)))))

(fn `UserConstructionScript`)