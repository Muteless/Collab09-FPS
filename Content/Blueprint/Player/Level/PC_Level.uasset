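; Level player controller that routes player input to the controlled pawn and creates the HUD.
; On BeginPlay it adds an Enhanced Input mapping context, and on possession it spawns the HUD widget with the character's Ability System Component.
; Move, look, jump, dash, primary and secondary action, and reload inputs are forwarded as messages carrying input type and value, leaving gameplay logic to the pawn.
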(event `self.ReceiveBeginPlay`
  (`self.AddMappingContext`))

(event `AddMappingContext`
  (`EnhancedInputSubsystemInterface.AddMappingContext` (subsystem `EnhancedInputLocalPlayerSubsystem`) (`self.InputMappingContext`) 0 (struct)))

(event `self.Possessed`
  (params (Character :type "CharacterBase Object Reference"))
  (bind _returnvalue (`AbilitySystemBlueprintLibrary.GetAbilitySystemComponent` Character))
  ;[1 0.03955 0.03955] Possessed
  ;[0 0.3916 0.8879] Create HUD
  (bind _returnvalue_2 (`|CreateWidget` "/Game/UI/HUD/WB_HUD.WB_HUD_C" self _returnvalue))
  (`/Game/UI/HUD/WB_HUD.Initialize` _returnvalue_2 _returnvalue)
  (`UserWidget.AddToViewport` _returnvalue_2 0))

(event `EnhancedInput|/Game/Input/InputActions/IA_PrimaryAction`
  (params (ActionValue :type Boolean) (ElapsedSeconds :type "Float (double-precision)") (TriggeredSeconds :type "Float (double-precision)") (InputAction :type "InputAction Object Reference" :default "/Game/Input/InputActions/IA_PrimaryAction.IA_PrimaryAction"))
  ;[1 0.03955 0.03955] IA_PrimaryAction
  (:`Started`
    (message `CharacterInput.InputActionPrimaryAction` (`self.K2_GetPawn`) "Started" ActionValue)))

(event `EnhancedInput|/Game/Input/InputActions/IA_Jump`
  (params (ActionValue :type Boolean) (ElapsedSeconds :type "Float (double-precision)") (TriggeredSeconds :type "Float (double-precision)") (InputAction :type "InputAction Object Reference" :default "/Game/Input/InputActions/IA_Jump.IA_Jump"))
  (bind _returnvalue (`self.K2_GetPawn`))
  ;[1 0.03955 0.03955] IA_Jump
  (:`Started`
    (message `CharacterInput.InputActionJump` _returnvalue "Started" ActionValue))
  (:`Canceled`
    (message `CharacterInput.InputActionJump` _returnvalue "Completed" ActionValue :!label _label))
  (:`Completed`
    (goto _label)))

(event `EnhancedInput|/Game/Input/InputActions/IA_Dash`
  (params (ActionValue :type Boolean) (ElapsedSeconds :type "Float (double-precision)") (TriggeredSeconds :type "Float (double-precision)") (InputAction :type "InputAction Object Reference" :default "/Game/Input/InputActions/IA_Dash.IA_Dash"))
  ;[1 0.03955 0.03955] IA_Dash
  (:`Started`
    (message `CharacterInput.InputActionDash` (`self.K2_GetPawn`) "Started" ActionValue)))

(event `EnhancedInput|/Game/Input/InputActions/IA_Move`
  (params (ActionValue :type "Vector2D Structure") (ElapsedSeconds :type "Float (double-precision)") (TriggeredSeconds :type "Float (double-precision)") (InputAction :type "InputAction Object Reference" :default "/Game/Input/InputActions/IA_Move.IA_Move"))
  ;[1 0.03955 0.03955] IA_Move
  (:`Triggered`
    (message `CharacterInput.InputActionMove` (`self.K2_GetPawn`) "Triggered" ActionValue)))

(event `EnhancedInput|/Game/Input/InputActions/IA_SecondaryAction`
  (params (ActionValue :type Boolean) (ElapsedSeconds :type "Float (double-precision)") (TriggeredSeconds :type "Float (double-precision)") (InputAction :type "InputAction Object Reference" :default "/Game/Input/InputActions/IA_SecondaryAction.IA_SecondaryAction"))
  ;[1 0.03955 0.03955] IA_SecondaryAction
  (:`Started`
    (message `CharacterInput.InputActionSecondaryAction` (`self.K2_GetPawn`) "Started" ActionValue)))

(event `EnhancedInput|/Game/Input/InputActions/IA_Reload`
  (params (ActionValue :type Boolean) (ElapsedSeconds :type "Float (double-precision)") (TriggeredSeconds :type "Float (double-precision)") (InputAction :type "InputAction Object Reference" :default "/Game/Input/InputActions/IA_Reload.IA_Reload"))
  ;[1 0.03955 0.03955] IA_Reload
  (:`Started`
    (message `CharacterInput.InputActionReload` (`self.K2_GetPawn`) "Started" ActionValue)))

(event `EnhancedInput|/Game/Input/InputActions/IA_Look`
  (params (ActionValue :type "Vector2D Structure") (ElapsedSeconds :type "Float (double-precision)") (TriggeredSeconds :type "Float (double-precision)") (InputAction :type "InputAction Object Reference" :default "/Game/Input/InputActions/IA_Look.IA_Look"))
  ;[1 0.03955 0.03955] IA_Look
  (:`Triggered`
    (message `CharacterInput.InputActionLook` (`self.K2_GetPawn`) "Triggered" ActionValue)))

(fn `UserConstructionScript`)