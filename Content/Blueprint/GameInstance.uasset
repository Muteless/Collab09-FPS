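; Game Instance Blueprint that handles animated transitions between levels.
; TransitionLevel stores the world index, looks up the target PersistentWorld through GetLevelData, then shows a WB_LevelTransition widget and starts it with a finished-playing callback bound.
; TransitionWorldAnimationFinished opens the stored world by object reference and sets game-only input mode.
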(event `GameInstanceInterface.TransitionLevel`
  (params (WorldIndex :type Integer))
  ;[0.9387 0.0382 0.0382] Transition World
  (set `self.WorldIndex` WorldIndex)
  (bind _returnvalue (`GameInstanceInterface.GetLevelData`))
  (set `self.WorldToTransitionTo` (`LevelDataAsset.PersistentWorld` _returnvalue))
  (bind _returnvalue_2 (`|CreateWidget` "/Game/UI/Transitions/WB_LevelTransition.WB_LevelTransition_C" (`GameplayStatics.GetPlayerController` 0)))
  (bind _output_get (set `self.LevelTransitionWidget` _returnvalue_2))
  (`UserWidget.AddToViewport` _output_get 0)
  (add `/Game/UI/Transitions/WB_LevelTransition.ED_FinishedPlaying` _output_get (`|CreateDelegate` :!event `TransitionWorldAnimationFinished`))
  (`/Game/UI/Transitions/WB_LevelTransition.BeginPlay` _output_get false))

(event `TransitionWorldAnimationFinished`
  ;[0.9387 0.0382 0.0382] Transition World
  (`GameplayStatics.OpenLevelBySoftObjectPtr` (`self.WorldToTransitionTo`))
  (`WidgetBlueprintLibrary.SetInputMode_GameOnly` (`GameplayStatics.GetPlayerController` 0)))