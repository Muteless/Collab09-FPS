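; BP_DeepSeek is a test AI character that visualizes a Blackboard location for debugging.
; On BeginPlay it prints the class name of its CharacterMovement component.
; Each Tick it casts its controller to ChatGPT, reads the TestPoint vector from that controller's Blackboard and draws a red debug sphere there.
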(event `self.ReceiveBeginPlay`
  (`KismetSystemLibrary.PrintString` (`KismetSystemLibrary.GetClassDisplayName` (`GameplayStatics.GetObjectClass` (`self.CharacterMovement`)))))

(event `self.ReceiveTick`
  (params (DeltaSeconds :type "Float (single-precision)"))
  (bind _aschat_gpt (cast `/Game/Blueprint/AI/EnemyAI/TestAI/ChatGPT` (`self.GetController`)))
  (`KismetSystemLibrary.DrawDebugSphere` (`BlackboardComponent.GetValueAsVector` (`BaseAI.BlackboardComponent` _aschat_gpt) (`KismetStringLibrary.Conv_StringToName` "TestPoint")) 30.0 12 (struct :`R` 1.0 :`A` 1.0)))

(fn `UserConstructionScript`)