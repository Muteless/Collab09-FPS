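; BP_Normal_Support is the normal Support enemy pawn, caching its AIC_Normal_Support controller on possession.
; Every Tick it compares its distance to the blackboard's V_TargetPosition against a fixed radius and writes two opposite booleans.
; Despite its name, B_IsAtTargetLocation is true outside that radius, while its Invert twin is true inside.
; NiagaraEnable briefly shows a Niagara effect, then hides it.
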(event `self.ReceiveTick`
  (params (DeltaSeconds :type "Float (single-precision)"))
  (bind _returnvalue (`AIBlueprintHelperLibrary.GetBlackboard` (`self.NewController`)))
  (bind _returnvalue_2 (<= (`KismetMathLibrary.Vector_Distance` (`BlackboardComponent.GetValueAsVector` _returnvalue (`KismetStringLibrary.Conv_StringToName` "V_TargetPosition")) (`self.K2_GetActorLocation`)) 500.0))
  (`/Engine/EditorBlueprintResources/StandardMacros.IsValid` (`self.NewController`)
    (:`Is Valid`
      (`BlackboardComponent.SetValueAsBool` _returnvalue (`KismetStringLibrary.Conv_StringToName` "B_IsAtTargetLocation") (not _returnvalue_2))
      (`BlackboardComponent.SetValueAsBool` _returnvalue (`KismetStringLibrary.Conv_StringToName` "B_IsAtTargetLocationInvert") _returnvalue_2))))

(event `self.ReceivePossessed`
  (params (NewController :type "Controller Object Reference"))
  (bind _asaic_normal_support (cast `/Game/Blueprint/AI/EnemyTypes/Support/Normal/AIC_Normal_Support` NewController))
  (set `self.NewController` _asaic_normal_support))

(event `NiagaraEnable`
  (bind _niagara (`self.Niagara`))
  (`SceneComponent.SetVisibility` _niagara true false)
  (`KismetSystemLibrary.Delay` 1.0)
  (`SceneComponent.SetVisibility` _niagara false false))

(fn `UserConstructionScript`
  (`parent.UserConstructionScript`))