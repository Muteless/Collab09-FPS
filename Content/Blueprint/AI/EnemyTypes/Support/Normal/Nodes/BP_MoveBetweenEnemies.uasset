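; Behavior tree task for the normal Support enemy that picks a target position amid nearby BP_DeepSeek actors.
; It averages the locations of those actors overlapping the pawn's HealAura, projects that centroid onto the navmesh and writes it to the V_TargetPosition blackboard key.
; It only sets the position, and fails when a cast fails or none of those actors are in the aura.
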(event `self.ReceiveExecute`
  (params (OwnerActor :type "Actor Object Reference"))
  (bind _sumvec (`self.SumVec`))
  (bind _asaic_normal_support (cast `/Game/Blueprint/AI/EnemyTypes/Support/Normal/AIC_Normal_Support` (`AIBlueprintHelperLibrary.GetAIController` OwnerActor))
    (:`then`
      (bind _asbp_normal_support (cast `/Game/Blueprint/AI/EnemyTypes/Support/Normal/BP_Normal_Support` (`Controller.K2_GetPawn` _asaic_normal_support))
        (:`then`
          (bind _output_get (set `self.SelfAsBP` _asbp_normal_support))
          (bind _overlappingactors (`PrimitiveComponent.GetOverlappingActors` (`/Game/Blueprint/AI/EnemyTypes/Support/Normal/BP_Normal_Support.HealAura` _output_get) "/Game/Blueprint/AI/EnemyAI/TestAI/BP_DeepSeek.BP_DeepSeek_C"))
          (bind _returnvalue (`KismetArrayLibrary.Array_Length` _overlappingactors))
          (if (> _returnvalue 0)
            (for _array_element _overlappingactors
              (set `self.SumVec` (+ _sumvec (`Actor.K2_GetActorLocation` _array_element))))
            (`BlackboardComponent.SetValueAsVector` (`AIBlueprintHelperLibrary.GetBlackboard` _asbp_normal_support) (`KismetStringLibrary.Conv_StringToName` "V_TargetPosition") (`NavigationSystemV1.K2_ProjectPointToNavigation` (/ _sumvec _returnvalue) null null (300.0 300.0 300.0)))
            (`KismetSystemLibrary.PrintString` (`KismetStringLibrary.Conv_VectorToString` (0.0 0.0 0.0)) false false)
            (set `self.SumVec` (0.0 0.0 0.0))
            (`self.FinishExecute` true)
            (else
              (`self.FinishExecute` false))))
        (:`CastFailed`
          (`self.FinishExecute` false :!label _label))))
    (:`CastFailed`
      (goto _label))))