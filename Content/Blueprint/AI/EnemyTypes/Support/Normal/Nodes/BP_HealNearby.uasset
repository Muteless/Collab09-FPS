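; Behavior tree task that makes a Normal Support enemy heal BP_DeepSeek actors around it.
; It enables the pawn's Niagara effect, then gathers overlapping actors from its HealAura.
; Each target's own ability system applies GE_Heal to itself, with a fixed amount passed as a set-by-caller magnitude.
; The task succeeds after the heal pass and fails if the controller or pawn cast fails.
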(event `self.ReceiveExecute`
  (params (OwnerActor :type "Actor Object Reference"))
  (bind _asaic_normal_support (cast `/Game/Blueprint/AI/EnemyTypes/Support/Normal/AIC_Normal_Support` (`AIBlueprintHelperLibrary.GetAIController` OwnerActor))
    (:`then`
      (bind _asbp_normal_support (cast `/Game/Blueprint/AI/EnemyTypes/Support/Normal/BP_Normal_Support` (`Controller.K2_GetPawn` _asaic_normal_support))
        (:`then`
          (bind _output_get (set `self.SelfAsBP` _asbp_normal_support))
          (`/Game/Blueprint/AI/EnemyTypes/Support/Normal/BP_Normal_Support.NiagaraEnable` _output_get)
          (bind _overlappingactors (`PrimitiveComponent.GetOverlappingActors` (`/Game/Blueprint/AI/EnemyTypes/Support/Normal/BP_Normal_Support.HealAura` _output_get) "/Game/Blueprint/AI/EnemyAI/TestAI/BP_DeepSeek.BP_DeepSeek_C"))
          (`KismetArrayLibrary.Array_RemoveItem` _overlappingactors OwnerActor)
          (if (not (> 0 (`KismetArrayLibrary.Array_Length` _overlappingactors)))
            (for _array_element _overlappingactors
              (bind _returnvalue (`AbilitySystemBlueprintLibrary.GetAbilitySystemComponent` _array_element))
              (bind _output_get_2 (set `self.Context` (`AbilitySystemComponent.MakeEffectContext` _returnvalue)))
              (`AbilitySystemBlueprintLibrary.EffectContextAddHitResult` _output_get_2 (struct) true)
              (bind _returnvalue_2 (`AbilitySystemBlueprintLibrary.AssignTagSetByCallerMagnitude` (`AbilitySystemComponent.MakeOutgoingSpec` _returnvalue "/Game/Blueprint/GAS/Effects/GE_Heal.GE_Heal_C" 0.0 _output_get_2) (struct :`TagName` "Data.Magnitude") 100.0))
              (`AbilitySystemComponent.BP_ApplyGameplayEffectSpecToSelf` _returnvalue _returnvalue_2)))
          (`self.FinishExecute` true))
        (:`CastFailed`
          (`self.FinishExecute` false :!label _label))))
    (:`CastFailed`
      (goto _label))))