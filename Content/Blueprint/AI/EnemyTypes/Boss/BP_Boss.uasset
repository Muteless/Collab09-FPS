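; BP_Boss is the boss enemy, with health-style phase tracking, minion spawning and a brief Niagara effect.
; Tick compares two ability system attribute values and, below half, sets "Phase One Complete" on the blackboard of the AIC_Boss cached at possession, printing debug text.
; SpawnEnemies has each spawner create a random enemy type set to auto-target the player.
; NiagaraEnable briefly shows the effect, then hides it.
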(event `self.ReceiveTick`
  (params (DeltaSeconds :type "Float (single-precision)"))
  (bind _abilitysystemcomponent (`self.AbilitySystemComponent`))
  (if (>= (`.ReturnValue` (`AbilitySystemComponent.GetGameplayAttributeValue` _abilitysystemcomponent (struct :`AttributeName` "CurrentHealth" :`Attribute` "/Script/Collab09FPS.HealthAttributeSet:CurrentHealth" :`AttributeOwner` "/Script/CoreUObject.Class'/Script/Collab09FPS.HealthAttributeSet'"))) (/ (`.ReturnValue` (`AbilitySystemComponent.GetGameplayAttributeValue` _abilitysystemcomponent (struct :`AttributeName` "MaxHealth" :`Attribute` "/Script/Collab09FPS.HealthAttributeSet:MaxHealth" :`AttributeOwner` "/Script/CoreUObject.Class'/Script/Collab09FPS.HealthAttributeSet'"))) 2.0))
    (`KismetSystemLibrary.PrintString` "Above half" false false)
    (else
      (`KismetSystemLibrary.PrintString` "Below half" false false)
      (`BlackboardComponent.SetValueAsBool` (`AIBlueprintHelperLibrary.GetBlackboard` (`self.Boss`)) (`KismetStringLibrary.Conv_StringToName` "Phase One Complete") true))))

(event `self.ReceivePossessed`
  (params (NewController :type "Controller Object Reference"))
  (bind _asaic_boss (cast `/Game/Blueprint/AI/EnemyTypes/Boss/AIC_Boss` NewController))
  (set `self.Boss` _asaic_boss))

(event `Spawn Enemies`
  (for _array_element (`self.Spawners`)
    (set `AISpawner.EnemyStartBehaviour` "AutoTargetPlayer" _array_element)
    (set `AISpawner.Enemy` (cast `EEnemyTypes` (`KismetMathLibrary.Conv_IntToByte` (`KismetMathLibrary.RandomIntegerInRange` 1 3))) _array_element)
    (`AISpawner.SpawnEnemy` _array_element)))

(event `NiagaraEnable`
  (bind _niagara (`self.Niagara`))
  (`SceneComponent.SetVisibility` _niagara true false)
  (`KismetSystemLibrary.Delay` 0.56)
  (`SceneComponent.SetVisibility` _niagara false false))

(fn `UserConstructionScript`)