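; Behavior tree task for the boss's projectile attack, firing a staggered five-shot volley at the player.
; On execute it reads the player from the blackboard, yaws the boss toward the player's camera and computes one aim rotation from Arrow1.
; Three functions spawn projectiles from the boss's arrow components in short-delayed waves of one, two and two, all sharing that rotation.
; Failed boss or controller casts never finish the task.
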(event `self.ReceiveTick`
  (params (OwnerActor :type "Actor Object Reference") (DeltaSeconds :type "Float (single-precision)"))
  (set `self.SpinDurationElapsed` (+ DeltaSeconds (`self.SpinDurationElapsed`))))

(event `self.ReceiveExecute`
  (params (OwnerActor :type "Actor Object Reference"))
  (bind _returnvalue (`SceneComponent.K2_GetComponentLocation` (`PlayerCharacterBase.CameraComponent` (`self.Player`))))
  (bind _returnvalue_2 (`SceneComponent.K2_GetComponentLocation` (`/Game/Blueprint/AI/EnemyAI/TestAI/BP_DeepSeek.Arrow1` (`self.SelfAsBP`))))
  (bind (_returnvalue_roll _returnvalue_pitch _returnvalue_yaw) (`KismetMathLibrary.BreakRotator` (`KismetMathLibrary.FindLookAtRotation` _returnvalue_2 _returnvalue)))
  (bind _asaicontroller (cast `AIController` OwnerActor)
    (:`then`
      (bind _asbp_boss (cast `/Game/Blueprint/AI/EnemyTypes/Boss/BP_Boss` (`Controller.K2_GetPawn` _asaicontroller))
        (:`then`
          (set `self.SelfAsBP` _asbp_boss)
          (bind _asplayer_character (cast `/Game/Blueprint/Player/Level/PlayerCharacter` (`BlackboardComponent.GetValueAsObject` (`AIBlueprintHelperLibrary.GetBlackboard` OwnerActor) (`KismetStringLibrary.Conv_StringToName` "O_PlayerObject")))
            (:`then`
              (set `self.Player` _asplayer_character)
              (set `self.DirectionRotator` (`KismetMathLibrary.Conv_VectorToRotator` (- _returnvalue _returnvalue_2)))
              (`Actor.K2_SetActorRotation` (`self.SelfAsBP`) (`KismetMathLibrary.MakeRotator` 0.0 0.0 _returnvalue_yaw) false)
              (`self.Projectile 1` (`self.DirectionRotator`))
              (`KismetSystemLibrary.Delay` 0.1)
              (`self.Projectile 2` (`self.DirectionRotator`))
              (`KismetSystemLibrary.Delay` 0.1)
              (`self.Projectile 3` (`self.DirectionRotator`))
              (`self.FinishExecute` true))
            (:`CastFailed`
              (`KismetSystemLibrary.PrintString` "Hello")
              (`self.FinishExecute` false))))
        (:`CastFailed`
          (`KismetSystemLibrary.PrintString` "Cast to BP_DeekSeek failed"))))
    (:`CastFailed`
      (`KismetSystemLibrary.PrintString` "Cast to AIC failed" false false))))

(fn `Projectile 1`
  (params (InXRotator :type "Rotator Structure"))
  (`KismetSystemLibrary.PrintString` "Bang Line 1" true false)
  (`|SpawnActorFromClass` (`self.Projectile`) (`KismetMathLibrary.MakeTransform` (`SceneComponent.K2_GetComponentLocation` (`/Game/Blueprint/AI/EnemyAI/TestAI/BP_DeepSeek.Arrow1` (`self.SelfAsBP`))) InXRotator) "AlwaysSpawn" "MultiplyWithRoot" (`self.SelfAsBP`) null))

(fn `Projectile 2`
  (params (InXRotator :type "Rotator Structure"))
  (bind _selfasbp (`self.SelfAsBP`))
  (bind _selfasbp_2 (`self.SelfAsBP`))
  (bind _projectile (`self.Projectile`))
  (`KismetSystemLibrary.PrintString` "Bang Line 2" true false)
  (`|SpawnActorFromClass` _projectile (`KismetMathLibrary.MakeTransform` (`SceneComponent.K2_GetComponentLocation` (`/Game/Blueprint/AI/EnemyTypes/Boss/BP_Boss.Arrow3` _selfasbp)) InXRotator) "AlwaysSpawn" "MultiplyWithRoot" _selfasbp_2 _selfasbp_2)
  (`|SpawnActorFromClass` _projectile (`KismetMathLibrary.MakeTransform` (`SceneComponent.K2_GetComponentLocation` (`/Game/Blueprint/AI/EnemyTypes/Boss/BP_Boss.Arrow2` _selfasbp)) InXRotator) "AlwaysSpawn" "MultiplyWithRoot" _selfasbp_2 _selfasbp_2))

(fn `Projectile 3`
  (params (InXRotator :type "Rotator Structure"))
  (bind _selfasbp (`self.SelfAsBP`))
  (bind _selfasbp_2 (`self.SelfAsBP`))
  (bind _projectile (`self.Projectile`))
  (`KismetSystemLibrary.PrintString` "Bang Line 2" true false)
  (`|SpawnActorFromClass` _projectile (`KismetMathLibrary.MakeTransform` (`SceneComponent.K2_GetComponentLocation` (`/Game/Blueprint/AI/EnemyTypes/Boss/BP_Boss.Arrow4` _selfasbp)) InXRotator) "AlwaysSpawn" "MultiplyWithRoot" _selfasbp_2 _selfasbp_2)
  (`|SpawnActorFromClass` _projectile (`KismetMathLibrary.MakeTransform` (`SceneComponent.K2_GetComponentLocation` (`/Game/Blueprint/AI/EnemyTypes/Boss/BP_Boss.Arrow5` _selfasbp)) InXRotator) "AlwaysSpawn" "MultiplyWithRoot" _selfasbp_2 _selfasbp_2))