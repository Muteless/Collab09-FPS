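; Behavior tree task for the boss's AOE attack, which knocks back and damages the player.
; It takes the player from the blackboard and hits only if they overlap both the boss's Sphere and Box, succeeding even on a miss.
; Hits apply root-motion impulse and damage GameplayEffects with set-by-caller magnitudes, passing an away-from-boss, upward-tilted direction through the hit result normal.
; An older capsule-overlap version remains as unreachable nodes.
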(event `CheckCollision`
  (bind _actor (`self.Actor`))
  (bind _player (`self.Player`))
  (bind _returnvalue (`AbilitySystemBlueprintLibrary.GetAbilitySystemComponent` (`self.Player`)))
  (bind (_returnvalue_x _returnvalue_y) (`KismetMathLibrary.BreakVector` (- (`Actor.K2_GetActorLocation` (`self.Player`)) (`Actor.K2_GetActorLocation` (`self.Actor`)))))
  (bind (_returnvalue_x_2 _returnvalue_y_2) (`KismetMathLibrary.BreakVector` (`KismetMathLibrary.Normal` (`KismetMathLibrary.MakeVector` _returnvalue_x _returnvalue_y 250.0))))
  (if (`KismetArrayLibrary.Array_Contains` (`PrimitiveComponent.GetOverlappingActors` (`/Game/Blueprint/AI/EnemyTypes/Boss/BP_Boss.Sphere` _actor) null) _player)
    (if (`KismetArrayLibrary.Array_Contains` (`PrimitiveComponent.GetOverlappingActors` (`/Game/Blueprint/AI/EnemyTypes/Boss/BP_Boss.Box` _actor) null) _player)
      (bind _output_get (set `self.Context` (`AbilitySystemComponent.MakeEffectContext` _returnvalue)))
      (`AbilitySystemBlueprintLibrary.EffectContextAddHitResult` _output_get (`GameplayStatics.MakeHitResult` false false 0.0 0.0 (0.0 0.0 0.0) (0.0 0.0 0.0) (`KismetMathLibrary.MakeVector` _returnvalue_x_2 _returnvalue_y_2 0.5)) true)
      (bind _returnvalue_2 (`AbilitySystemBlueprintLibrary.AssignTagSetByCallerMagnitude` (`AbilitySystemComponent.MakeOutgoingSpec` _returnvalue "/Game/Blueprint/GAS/Effects/Movement/GE_RootMotionImpulse.GE_RootMotionImpulse_C" 0.0 _output_get) (struct :`TagName` "Data.Magnitude") (`self.Knockback`)))
      (`AbilitySystemComponent.BP_ApplyGameplayEffectSpecToSelf` _returnvalue _returnvalue_2)
      (bind _returnvalue_3 (`AbilitySystemBlueprintLibrary.AssignTagSetByCallerMagnitude` (`AbilitySystemComponent.MakeOutgoingSpec` _returnvalue "/Game/Blueprint/GAS/Effects/Damage/GE_Damage.GE_Damage_C" 0.0 _output_get) (struct :`TagName` "Data.Magnitude") (`self.Damage`)))
      (`AbilitySystemComponent.BP_ApplyGameplayEffectSpecToSelf` _returnvalue _returnvalue_3))))

(event `self.ReceiveExecute`
  (params (OwnerActor :type "Actor Object Reference"))
  (bind _asplayer_character (cast `/Game/Blueprint/Player/Level/PlayerCharacter` (`BlackboardComponent.GetValueAsObject` (`AIBlueprintHelperLibrary.GetBlackboard` OwnerActor) (`KismetStringLibrary.Conv_StringToName` "O_PlayerObject")))
    (:`then`
      (set `self.Player` _asplayer_character)
      (bind _asaicontroller (cast `AIController` OwnerActor))
      (bind _asbp_boss (cast `/Game/Blueprint/AI/EnemyTypes/Boss/BP_Boss` (`Controller.K2_GetPawn` _asaicontroller))
        (:`then`
          (set `self.Actor` _asbp_boss)
          (`self.CheckCollision`)
          (`self.FinishExecute` true))
        (:`CastFailed`
          (`self.FinishExecute` false))))
    (:`CastFailed`
      (`self.FinishExecute` false))))