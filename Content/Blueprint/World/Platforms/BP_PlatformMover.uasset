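; BP_PlatformMover moves its attached actors along the PlatformRoute spline as moving platforms.
; MovementType selects constant back-and-forth motion or a start when Box is overlapped, while trigger interface events drive it forward or in reverse.
; A timeline samples the spline at constant velocity to position actors and Box, with play rate scaled from Speed and spline length.
; Ending a Box overlap stops the timeline.
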(event `self.ReceiveBeginPlay`
  (set `self.AttachedPlatform` (`self.GetAttachedActors` true))
  (switch `/Game/Enumeration/E_PlatformType` (`self.MovementType`)
    (:`NewEnumerator1`
      (`self.Move` false))))

(event `self.Box.OnComponentBeginOverlap`
  (params (OverlappedComponent :type "PrimitiveComponent Object Reference") (OtherActor :type "Actor Object Reference") (OtherComp :type "PrimitiveComponent Object Reference") (OtherBodyIndex :type Integer) (bFromSweep :type Boolean) (SweepResult :type "HitResult Structure (by ref)"))
  (switch `/Game/Enumeration/E_PlatformType` (`self.MovementType`)
    (:`NewEnumerator0`
      (`self.Move` false))))

(event `Move`
  (params (Reverse :type Boolean))
  (for _array_element (`self.AttachedPlatform`)
    (if Reverse
      (bind (_direction _splineposition) (`Timeline|TL_Movement` :!via `Reverse` :!label _label)
        (:`Update`
          (bind _returnvalue (`SplineComponent.GetLocationAtTime` (`self.Platform Route`) _splineposition "World" true))
          (`self.K2_SetActorLocation` _array_element _returnvalue false false)
          (`SceneComponent.K2_SetWorldLocation` (`self.Box`) _returnvalue false false))
        (:`Finished`
          (switch `/Game/Enumeration/E_PlatformType` (`self.MovementType`)
            (:`NewEnumerator1`
              (`self.Move` (not Reverse))))))
      (else
        (goto _label)))))

(event `self.Box.OnComponentEndOverlap`
  (params (OverlappedComponent :type "PrimitiveComponent Object Reference") (OtherActor :type "Actor Object Reference") (OtherComp :type "PrimitiveComponent Object Reference") (OtherBodyIndex :type Integer))
  (goto _label :!via `Stop`))

(event `/Game/Blueprint/Interface/BPI_Trigger.I_StartTrigger`
  (params (Instigator :type "/Game/Blueprint/World/Platforms/BP_Trigger Object Reference"))
  (`self.Move` false))

(event `/Game/Blueprint/Interface/BPI_Trigger.I_EndTrigger`
  (params (Instigator :type "/Game/Blueprint/World/Platforms/BP_Trigger Object Reference"))
  (`self.Move` true))

(fn `UserConstructionScript`
  (bind _output_get (set `self.SplineLength` (`SplineComponent.GetSplineLength` (`self.Platform Route`))))
  (`TimelineComponent.SetPlayRate` (`self.TL_Movement`) (/ (`self.Speed`) _output_get)))