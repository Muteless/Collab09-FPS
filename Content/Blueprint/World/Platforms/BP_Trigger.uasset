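; BP_Trigger is a trigger volume that sends start and end trigger messages to a configured list of actors.
; By default, overlapping the box sends the start message and leaving it sends the end message, each passing the trigger as the sender.
; With Toggleable set, a FlipFlop alternates start and end on successive overlaps, and leaving the box does nothing.
; Only the start loop checks that each actor is valid.
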(event `self.Box.OnComponentBeginOverlap`
  (params (OverlappedComponent :type "PrimitiveComponent Object Reference") (OtherActor :type "Actor Object Reference") (OtherComp :type "PrimitiveComponent Object Reference") (OtherBodyIndex :type Integer) (bFromSweep :type Boolean) (SweepResult :type "HitResult Structure (by ref)"))
  (if (`self.Toggleable?`)
    (`/Engine/EditorBlueprintResources/StandardMacros.FlipFlop`
      (:`A`
        (for _array_element (`self.Actors`) :!label _label
          (`/Engine/EditorBlueprintResources/StandardMacros.IsValid` _array_element
            (:`Is Valid`
              (message `/Game/Blueprint/Interfaces/BPI_Trigger.I_StartTrigger` _array_element self)))))
      (:`B`
        (for _array_element_2 (`self.Actors`) :!label _label_2
          (message `/Game/Blueprint/Interfaces/BPI_Trigger.I_EndTrigger` _array_element_2 self))))
    (else
      (goto _label))))

(event `self.Box.OnComponentEndOverlap`
  (params (OverlappedComponent :type "PrimitiveComponent Object Reference") (OtherActor :type "Actor Object Reference") (OtherComp :type "PrimitiveComponent Object Reference") (OtherBodyIndex :type Integer))
  (if (not (`self.Toggleable?`))
    (goto _label_2)))

(fn `UserConstructionScript`)