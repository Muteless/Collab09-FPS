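; Teleporter is a world actor that moves player characters to a set destination when they overlap its collision component.
; It acts only while enabled, toggled through IEnable and IDisable events, and identifies players by a gameplay tag on their ability system component.
; The player lands at the TeleportPoint location, with both actor and controller rotation aligned to the Arrow component.
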(event `self.CollisionComponent.OnComponentBeginOverlap`
  (params (OverlappedComponent :type "PrimitiveComponent Object Reference") (OtherActor :type "Actor Object Reference") (OtherComp :type "PrimitiveComponent Object Reference") (OtherBodyIndex :type Integer) (bFromSweep :type Boolean) (SweepResult :type "HitResult Structure (by ref)"))
  (bind _returnvalue (`SceneComponent.K2_GetComponentRotation` (`self.Arrow`)))
  (if (`self.Enabled`)
    (if (`GameplayTagAssetInterface.HasMatchingGameplayTag` (`AbilitySystemBlueprintLibrary.GetAbilitySystemComponent` OtherActor) (struct :`TagName` "Effect.PlayerCharacter"))
      (`self.K2_SetActorLocationAndRotation` OtherActor (`SceneComponent.K2_GetComponentLocation` (`self.TeleportPoint`)) _returnvalue false false)
      (`Controller.SetControlRotation` (`self.GetInstigatorController` OtherActor) _returnvalue))))

(event `/Game/Blueprint/Interface/BPI_Trigger.I_Enable`
  (set `self.Enabled` true))

(event `/Game/Blueprint/Interface/BPI_Trigger.I_Disable`
  (set `self.Enabled` false))

(fn `UserConstructionScript`)