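; A world trigger volume that shows a tooltip message on the HUD when a player character enters it.
; Begin overlap identifies the player by an ability system gameplay tag, then sends the text to its instigator controller through HUD interface calls.
; DisplayMode decides removal: Overlap hides the tooltip on any end overlap, while Timer hides it after a delay and destroys the volume.
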(event `self.CollisionComponent.OnComponentBeginOverlap`
  (params (OverlappedComponent :type "PrimitiveComponent Object Reference") (OtherActor :type "Actor Object Reference") (OtherComp :type "PrimitiveComponent Object Reference") (OtherBodyIndex :type Integer) (bFromSweep :type Boolean) (SweepResult :type "HitResult Structure (by ref)"))
  (if (`GameplayTagAssetInterface.HasMatchingGameplayTag` (`AbilitySystemBlueprintLibrary.GetAbilitySystemComponent` OtherActor) (struct :`TagName` "Effect.PlayerCharacter"))
    (bind _output_get (set `self.Controller` (`self.GetInstigatorController` OtherActor)))
    (message `/Game/Blueprint/Interface/BPI_HUD.I_HUD_SetToolTipText` _output_get (`self.Text`))
    (message `/Game/Blueprint/Interface/BPI_HUD.I_HUD_SetShowToolTip` _output_get true)
    (switch `/Game/Enumeration/E_TooltipDisplayMode` (`self.DisplayMode`)
      (:`NewEnumerator1`
        (bind _returnvalue (`KismetSystemLibrary.K2_SetTimerDelegate` (`|CreateDelegate` :!event `TimerEnded`) (`self.TimeBeforeGone`)))
        (set `self.TimerHandle` _returnvalue)))))

(event `self.CollisionComponent.OnComponentEndOverlap`
  (params (OverlappedComponent :type "PrimitiveComponent Object Reference") (OtherActor :type "Actor Object Reference") (OtherComp :type "PrimitiveComponent Object Reference") (OtherBodyIndex :type Integer))
  (switch `/Game/Enumeration/E_TooltipDisplayMode` (`self.DisplayMode`)
    (:`NewEnumerator0`
      (bind _controller (`self.Controller`)
        (:`then`
          (message `/Game/Blueprint/Interface/BPI_HUD.I_HUD_SetShowToolTip` _controller false))
        (:`else`)))))

(event `TimerEnded`
  (message `/Game/Blueprint/Interface/BPI_HUD.I_HUD_SetShowToolTip` (`self.Controller`) false)
  (`KismetSystemLibrary.K2_ClearAndInvalidateTimerHandle` (`self.TimerHandle`))
  (`self.K2_DestroyActor`))

(fn `UserConstructionScript`)