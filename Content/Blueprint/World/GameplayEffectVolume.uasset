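; A world volume that applies a map of Gameplay Effects to overlapping actors through their Ability System Component.
; In one-shot mode it applies the effects to the first overlapping player character, then destroys itself.
; Otherwise it tracks overlapping actors and reapplies effects on a looping timer, cleared when the volume empties.
; Each effect's mapped value is passed as a SetByCaller magnitude under the Data.Magnitude tag.
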(event `self.CollisionComponent.OnComponentBeginOverlap`
  (params (OverlappedComponent :type "PrimitiveComponent Object Reference") (OtherActor :type "Actor Object Reference") (OtherComp :type "PrimitiveComponent Object Reference") (OtherBodyIndex :type Integer) (bFromSweep :type Boolean) (SweepResult :type "HitResult Structure (by ref)"))
  (bind _tickspeed (`self.TickSpeed`))
  (if (`self.OneShot`)
    (bind _asbp_player_character (cast `/Game/Blueprint/Player/Level/BP_PlayerCharacter` OtherActor))
    (`self.ApplyEffects` _asbp_player_character)
    (`self.K2_DestroyActor`)
    (else
      (`KismetArrayLibrary.Array_AddUnique` (`self.Actors`) OtherActor)
      (if (`KismetSystemLibrary.K2_IsTimerActiveHandle` (`self.TimerHandle`))
        _
        (elif (> _tickspeed 0.0)
          (bind _returnvalue (`KismetSystemLibrary.K2_SetTimerDelegate` (`|CreateDelegate` :!event `ApplyEffectsToActors`) _tickspeed true))
          (set `self.TimerHandle` _returnvalue))))))

(event `ApplyEffectsToActors`
  (for _array_element (`self.Actors`)
    (`self.ApplyEffects` _array_element)))

(event `self.CollisionComponent.OnComponentEndOverlap`
  (params (OverlappedComponent :type "PrimitiveComponent Object Reference") (OtherActor :type "Actor Object Reference") (OtherComp :type "PrimitiveComponent Object Reference") (OtherBodyIndex :type Integer))
  (bind _actors (`self.Actors`))
  (`KismetArrayLibrary.Array_RemoveItem` _actors OtherActor)
  (if (`KismetArrayLibrary.Array_IsEmpty` _actors)
    (`KismetSystemLibrary.K2_ClearAndInvalidateTimerHandle` (`self.TimerHandle`))))

(fn `ApplyEffects`
  (params (`Other Actor` :type "Actor Object Reference"))
  (bind _returnvalue (`AbilitySystemBlueprintLibrary.GetAbilitySystemComponent` `Other Actor`))
  (bind _effects (`self.Effects`))
  (`/Engine/EditorBlueprintResources/StandardMacros.IsValid` _returnvalue
    (:`Is Valid`
      (bind _keys (`BlueprintMapLibrary.Map_Keys` _effects))
      (for _array_element _keys
        (bind _returnvalue_2 (`AbilitySystemBlueprintLibrary.AssignTagSetByCallerMagnitude` (`AbilitySystemComponent.MakeOutgoingSpec` _returnvalue _array_element 0.0 (`AbilitySystemComponent.MakeEffectContext` _returnvalue)) (struct :`TagName` "Data.Magnitude") (`BlueprintMapLibrary.Map_Find` _effects _array_element)))
        (`AbilitySystemComponent.BP_ApplyGameplayEffectSpecToSelf` _returnvalue _returnvalue_2)))
    (:`Is Not Valid`
      (`KismetSystemLibrary.PrintString` "Overlapping Actor's Ability System Component is invalid"))))

(fn `UserConstructionScript`)