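; A world volume that repeatedly applies Gameplay Effects to actors inside it, named as a constant-force zone.
; Overlaps maintain a target list and drive a looping timer at TickSpeed, cleared when the volume empties.
; ApplyEffects applies each mapped effect through the target's Ability System Component, using the map value as the Data.Magnitude SetByCaller.
; The Arrow's forward vector travels as the hit normal in the effect context, supplying direction.
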(event `self.CollisionComponent.OnComponentBeginOverlap`
  (params (OverlappedComponent :type "PrimitiveComponent Object Reference") (OtherActor :type "Actor Object Reference") (OtherComp :type "PrimitiveComponent Object Reference") (OtherBodyIndex :type Integer) (bFromSweep :type Boolean) (SweepResult :type "HitResult Structure (by ref)"))
  (`KismetArrayLibrary.Array_AddUnique` (`self.TargetActors`) OtherActor)
  (bind _returnvalue (`KismetSystemLibrary.K2_SetTimerDelegate` (`|CreateDelegate` :!event `ApplyEffects`) (`self.TickSpeed`) true))
  (set `self.TimerHandle` _returnvalue))

(event `self.CollisionComponent.OnComponentEndOverlap`
  (params (OverlappedComponent :type "PrimitiveComponent Object Reference") (OtherActor :type "Actor Object Reference") (OtherComp :type "PrimitiveComponent Object Reference") (OtherBodyIndex :type Integer))
  (bind _targetactors (`self.TargetActors`))
  (`KismetArrayLibrary.Array_RemoveItem` _targetactors OtherActor)
  (if (`KismetArrayLibrary.Array_IsEmpty` _targetactors)
    (`KismetSystemLibrary.K2_ClearAndInvalidateTimerHandle` (`self.TimerHandle`))))

(event `ApplyEffects`
  (bind _onoverlapgameplayeffects (`self.OnOverlapGameplayEffects`))
  (for _array_element (`self.TargetActors`)
    (bind _returnvalue (`AbilitySystemBlueprintLibrary.GetAbilitySystemComponent` _array_element))
    (`/Engine/EditorBlueprintResources/StandardMacros.IsValid` _returnvalue
      (:`Is Valid`
        (bind _keys (`BlueprintMapLibrary.Map_Keys` _onoverlapgameplayeffects))
        (for _array_element_2 _keys
          (if (`KismetSystemLibrary.IsValidClass` _array_element_2)
            (bind _output_get (set `self.Context` (`AbilitySystemComponent.MakeEffectContext` _returnvalue)))
            (`AbilitySystemBlueprintLibrary.EffectContextAddHitResult` _output_get (`GameplayStatics.MakeHitResult` false false 0.0 0.0 (0.0 0.0 0.0) (0.0 0.0 0.0) (`SceneComponent.GetForwardVector` (`self.Arrow`))) true)
            (bind _returnvalue_2 (`AbilitySystemBlueprintLibrary.AssignTagSetByCallerMagnitude` (`AbilitySystemComponent.MakeOutgoingSpec` _returnvalue _array_element_2 0.0 _output_get) (struct :`TagName` "Data.Magnitude") (`BlueprintMapLibrary.Map_Find` _onoverlapgameplayeffects _array_element_2)))
            (`AbilitySystemComponent.BP_ApplyGameplayEffectSpecToSelf` _returnvalue _returnvalue_2)))))))

(fn `UserConstructionScript`)