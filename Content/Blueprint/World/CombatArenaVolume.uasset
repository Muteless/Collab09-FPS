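; CombatArenaVolume is a world volume that puts player characters under combat arena gameplay effects while they are inside it.
; When an actor begins overlapping its collision component, it checks the actor's Ability System Component for the Effect.PlayerCharacter tag and calls ApplyEffects on a match.
; On end overlap, the same check removes all stacks of GE_CombatArena from that actor.
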(event `self.CollisionComponent.OnComponentBeginOverlap`
  (params (OverlappedComponent :type "PrimitiveComponent Object Reference") (OtherActor :type "Actor Object Reference") (OtherComp :type "PrimitiveComponent Object Reference") (OtherBodyIndex :type Integer) (bFromSweep :type Boolean) (SweepResult :type "HitResult Structure (by ref)"))
  (bind _returnvalue (`AbilitySystemBlueprintLibrary.GetAbilitySystemComponent` OtherActor))
  (`/Engine/EditorBlueprintResources/StandardMacros.IsValid` _returnvalue
    (:`Is Valid`
      (if (`GameplayTagAssetInterface.HasMatchingGameplayTag` _returnvalue (struct :`TagName` "Effect.PlayerCharacter"))
        (`self.ApplyEffects` OtherActor)))))

(event `self.CollisionComponent.OnComponentEndOverlap`
  (params (OverlappedComponent :type "PrimitiveComponent Object Reference") (OtherActor :type "Actor Object Reference") (OtherComp :type "PrimitiveComponent Object Reference") (OtherBodyIndex :type Integer))
  (bind _returnvalue (`AbilitySystemBlueprintLibrary.GetAbilitySystemComponent` OtherActor))
  (`/Engine/EditorBlueprintResources/StandardMacros.IsValid` _returnvalue
    (:`Is Valid`
      (if (`GameplayTagAssetInterface.HasMatchingGameplayTag` _returnvalue (struct :`TagName` "Effect.PlayerCharacter"))
        (`AbilitySystemComponent.RemoveActiveGameplayEffectBySourceEffect` _returnvalue "/Game/Blueprint/GAS/Effects/GE_CombatArena.GE_CombatArena_C" null -1)))))

(fn `UserConstructionScript`
  (`parent.UserConstructionScript`))