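; BP_PlatformMover moves the actors attached to it, intended as platforms, along its PlatformRoute spline.
; On BeginPlay it gathers directly attached actors and starts moving if MovementType is Constant.
; Move loops over them and plays one shared timeline, whose update sets the loop's current element to a world-space spline position.
; The construction script scales timeline play rate by Speed over spline length, keeping speed independent of route length.
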(event `self.ReceiveBeginPlay`
  (set `self.AttachedPlatform` (`self.GetAttachedActors` true))
  (switch `/Game/Enumeration/E_PlatformType` (`self.MovementType`)
    (:`NewEnumerator1`
      (`self.Move`))))

(event `Move`
  (for _array_element (`self.AttachedPlatform`)
    (bind (_direction _splineposition) (`Timeline|TL_Movement` :`NewTime` 0.0)
      (:`Update`
        (`self.K2_SetActorLocation` _array_element (`SplineComponent.GetLocationAtTime` (`self.Platform Route`) _splineposition "World" true) false false)))))

(fn `UserConstructionScript`
  (bind _output_get (set `self.SplineLength` (`SplineComponent.GetSplineLength` (`self.Platform Route`))))
  (`TimelineComponent.SetPlayRate` (`self.TL_Movement`) (/ (`self.Speed`) _output_get)))