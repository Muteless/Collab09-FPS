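; BP_SlidingDoor is a two-panel sliding door whose panels move apart in opposite directions along relative X.
; DoorMovement takes an alpha and lerps Door and DoorR from the shared StartLocation transform to equal, opposite offsets, keeping rotation and scale.
; The construction script calls its parent, and the event graph is empty, so nothing in this Blueprint drives the alpha.
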(fn `DoorMovement`
  (params (InputPin :type "Float (single-precision)"))
  (bind (_startlocation_location _startlocation_rotation _startlocation_scale) (`KismetMathLibrary.BreakTransform` (`self.StartLocation`)))
  (bind (_startlocation_location_2 _startlocation_rotation_2 _startlocation_scale_2) (`KismetMathLibrary.BreakTransform` (`self.StartLocation`)))
  (`SceneComponent.K2_SetRelativeTransform` (`self.Door`) (`KismetMathLibrary.MakeTransform` (`KismetMathLibrary.VLerp` _startlocation_location_2 (+ _startlocation_location_2 (-156.0 0.0 0.0)) InputPin) _startlocation_rotation_2 _startlocation_scale_2) false false)
  (`SceneComponent.K2_SetRelativeTransform` (`self.DoorR`) (`KismetMathLibrary.MakeTransform` (`KismetMathLibrary.VLerp` _startlocation_location (+ _startlocation_location (156.0 0.0 0.0)) InputPin) _startlocation_rotation _startlocation_scale) false false))

(fn `UserConstructionScript`
  (`parent.UserConstructionScript`))