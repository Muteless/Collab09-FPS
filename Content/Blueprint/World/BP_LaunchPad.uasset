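; BP_LaunchPad is a world pad that applies Gameplay Effects to any actor with an Ability System Component overlapping its Box.
; Each effect class in the OnOverlapGameplayEffects map is applied to that actor, with its mapped value passed as the Data.Magnitude SetByCaller magnitude.
; The Arrow's forward vector travels in the effect context as a hit-result normal, carrying the pad's direction to the effects.
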(event `self.Box.OnComponentBeginOverlap`
  (params (OverlappedComponent :type "PrimitiveComponent Object Reference") (OtherActor :type "Actor Object Reference") (OtherComp :type "PrimitiveComponent Object Reference") (OtherBodyIndex :type Integer) (bFromSweep :type Boolean) (SweepResult :type "HitResult Structure (by ref)"))
  (bind _returnvalue (`AbilitySystemBlueprintLibrary.GetAbilitySystemComponent` OtherActor))
  (bind _onoverlapgameplayeffects (`self.OnOverlapGameplayEffects`))
  (`/Engine/EditorBlueprintResources/StandardMacros.IsValid` _returnvalue
    (:`Is Valid`
      (bind _keys (`BlueprintMapLibrary.Map_Keys` _onoverlapgameplayeffects))
      (for _array_element _keys
        (if (`KismetSystemLibrary.IsValidClass` _array_element)
          (bind _output_get (set `self.Context` (`AbilitySystemComponent.MakeEffectContext` _returnvalue)))
          (`AbilitySystemBlueprintLibrary.EffectContextAddHitResult` _output_get (`GameplayStatics.MakeHitResult` false false 0.0 0.0 (0.0 0.0 0.0) (0.0 0.0 0.0) (`SceneComponent.GetForwardVector` (`self.Arrow`))) true)
          (bind _returnvalue_2 (`AbilitySystemBlueprintLibrary.AssignTagSetByCallerMagnitude` (`AbilitySystemComponent.MakeOutgoingSpec` _returnvalue _array_element 0.0 _output_get) (struct :`TagName` "Data.Magnitude") (`BlueprintMapLibrary.Map_Find` _onoverlapgameplayeffects _array_element)))
          (`AbilitySystemComponent.BP_ApplyGameplayEffectSpecToSelf` _returnvalue _returnvalue_2))))))

(fn `UserConstructionScript`)