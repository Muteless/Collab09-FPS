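; BP_Door is a world door that slides its cube upward for actors holding a matching key and lowers it when they leave.
; Box overlap begin and end events check the actor's Ability System Component for the Key gameplay tag, then play or reverse a timeline.
; The timeline lerps the cube's world Z between its starting height and a fixed raised offset, both cached in the construction script.
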(event `self.Box.OnComponentBeginOverlap`
  (params (OverlappedComponent :type "PrimitiveComponent Object Reference") (OtherActor :type "Actor Object Reference") (OtherComp :type "PrimitiveComponent Object Reference") (OtherBodyIndex :type Integer) (bFromSweep :type Boolean) (SweepResult :type "HitResult Structure (by ref)"))
  (bind _success (`self.KeyCheck` OtherActor))
  (if _success
    (`self.TriggerDoor` true)))

(event `self.Box.OnComponentEndOverlap`
  (params (OverlappedComponent :type "PrimitiveComponent Object Reference") (OtherActor :type "Actor Object Reference") (OtherComp :type "PrimitiveComponent Object Reference") (OtherBodyIndex :type Integer))
  (bind _success (`self.KeyCheck` OtherActor))
  (if _success
    (`self.TriggerDoor` false)))

(event `TriggerDoor`
  (params (Open :type Boolean))
  (bind _cube (`self.Cube`))
  (bind (_returnvalue_x _returnvalue_y) (`KismetMathLibrary.BreakVector` (`SceneComponent.K2_GetComponentLocation` _cube)))
  (if Open
    (bind (_direction _open) (`Timeline|Timeline` :!label _label)
      (:`Update`
        (`SceneComponent.K2_SetWorldLocation` _cube (`KismetMathLibrary.MakeVector` _returnvalue_x _returnvalue_y (`KismetMathLibrary.Lerp` (`self.StartLocation`) (`self.EndLocation`) _open)) false false)))
    (else
      (goto _label :!via `Reverse`))))

(fn `KeyCheck`
  (params (OtherActor :type "Actor Object Reference"))
  (returns (Success :type Boolean))
  (return (`GameplayTagAssetInterface.HasMatchingGameplayTag` (`AbilitySystemBlueprintLibrary.GetAbilitySystemComponent` OtherActor) (`self.Key`))))

(fn `UserConstructionScript`
  (bind (_returnvalue_x _returnvalue_y _returnvalue_z) (`KismetMathLibrary.BreakVector` (`SceneComponent.K2_GetComponentLocation` (`self.Cube`))))
  (bind _output_get (set `self.StartLocation` _returnvalue_z))
  (set `self.EndLocation` (+ _output_get 200.0)))