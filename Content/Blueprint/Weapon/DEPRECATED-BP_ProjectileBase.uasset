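; Deprecated base projectile actor that applies a map of Gameplay Effects to what it hits, then destroys itself.
; Construction sets movement speed, gravity and Niagara visuals; BeginPlay destroys projectiles without effects.
; Hits pass the actor to ApplyEffects, which sets Data.Magnitude by caller on its Ability System Component.
; Owner and projectile overlaps call ApplyEffects without a target, and DestroyOnHit=false is unimplemented, so it still destroys.
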(event `DestroyOnHitFalse`
  (`KismetSystemLibrary.PrintString` "CURRENTLY AN EMPTY FUNCTION, AND THE PROJECTILE STILL DESTROYS AFTER THIS")
  (`self.K2_DestroyActor`))

(event `self.CollsionHitbox.OnComponentBeginOverlap`
  (params (OverlappedComponent :type "PrimitiveComponent Object Reference") (OtherActor :type "Actor Object Reference") (OtherComp :type "PrimitiveComponent Object Reference") (OtherBodyIndex :type Integer) (bFromSweep :type Boolean) (SweepResult :type "HitResult Structure (by ref)"))
  (if (`self.bAffectsOwner`)
    (if (== OtherActor (`self.GetOwner`))
      (`self.ApplyEffects` null)))
  (if (`self.bAffectsProjectiles`)
    (if (`KismetSystemLibrary.DoesImplementInterface` OtherActor "/Game/Blueprint/Weapon/BPI_Projectile.BPI_Projectile_C")
      (`self.ApplyEffects` null))))

(event `self.CollsionHitbox.OnComponentHit`
  (params (HitComponent :type "PrimitiveComponent Object Reference") (OtherActor :type "Actor Object Reference") (OtherComp :type "PrimitiveComponent Object Reference") (NormalImpulse :type "Vector Structure") (Hit :type "HitResult Structure (by ref)"))
  (`self.ApplyEffects` OtherActor))

(event `self.ReceiveBeginPlay`
  (if (`BlueprintMapLibrary.Map_IsEmpty` (`self.Effects`))
    (`KismetSystemLibrary.PrintString` "Projectile contains no effects, so nothing happens.")
    (`self.K2_DestroyActor`)))

(fn `ApplyEffects`
  (params (`Other Actor` :type "Actor Object Reference"))
  (bind _returnvalue (`AbilitySystemBlueprintLibrary.GetAbilitySystemComponent` `Other Actor`))
  (bind _effects (`self.Effects`))
  (`/Engine/EditorBlueprintResources/StandardMacros.IsValid` _returnvalue
    (:`Is Valid`
      (bind _keys (`BlueprintMapLibrary.Map_Keys` _effects))
      (for _array_element _keys
        (bind _returnvalue_2 (`AbilitySystemBlueprintLibrary.AssignTagSetByCallerMagnitude` (`AbilitySystemComponent.MakeOutgoingSpec` _returnvalue _array_element 0.0 (`AbilitySystemComponent.MakeEffectContext` _returnvalue)) (struct :`TagName` "Data.Magnitude") (`BlueprintMapLibrary.Map_Find` _effects _array_element)))
        (`AbilitySystemComponent.BP_ApplyGameplayEffectSpecToSelf` _returnvalue _returnvalue_2)
        (if (not (`self.bDestroyOnHit`))
          (`self.DestroyOnHitFalse`))))
    (:`Is Not Valid`
      _))
  (`self.K2_DestroyActor`))

(fn `UserConstructionScript`
  (bind _projectilemovement (`self.ProjectileMovement`))
  (bind _speed (`self.Speed`))
  (set `ProjectileMovementComponent.MaxSpeed` _speed _projectilemovement)
  (set `ProjectileMovementComponent.InitialSpeed` _speed _projectilemovement)
  (set `ProjectileMovementComponent.ProjectileGravityScale` (`self.GravityModifier`) _projectilemovement)
  (`NiagaraComponent.SetAsset` (`self.Niagara`) (`self.NiagaraSystem`) true))