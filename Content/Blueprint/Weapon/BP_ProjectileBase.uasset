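; Base projectile Blueprint whose construction script sets projectile movement speed and gravity scale from its variables.
; The hitbox hit event only prints "HIT", and the overlap event is empty.
; An unconnected chain would skip the owner and BPI_Projectile actors, apply mapped Gameplay Effects to the target's Ability System with SetByCaller Data.Magnitude, and destroy the projectile.
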(event `self.CollsionHitbox.OnComponentBeginOverlap`
  (params (OverlappedComponent :type "PrimitiveComponent Object Reference") (OtherActor :type "Actor Object Reference") (OtherComp :type "PrimitiveComponent Object Reference") (OtherBodyIndex :type Integer) (bFromSweep :type Boolean) (SweepResult :type "HitResult Structure (by ref)")))

(event `self.CollsionHitbox.OnComponentHit`
  (params (HitComponent :type "PrimitiveComponent Object Reference") (OtherActor :type "Actor Object Reference") (OtherComp :type "PrimitiveComponent Object Reference") (NormalImpulse :type "Vector Structure") (Hit :type "HitResult Structure (by ref)"))
  (`KismetSystemLibrary.PrintString` "HIT"))

(fn `UserConstructionScript`
  (bind _projectilemovement (`self.ProjectileMovement`))
  (bind _fspeed (`self.fSpeed`))
  (set `ProjectileMovementComponent.MaxSpeed` _fspeed _projectilemovement)
  (set `ProjectileMovementComponent.InitialSpeed` _fspeed _projectilemovement)
  (set `ProjectileMovementComponent.ProjectileGravityScale` (`self.fGravityModifier`) _projectilemovement))