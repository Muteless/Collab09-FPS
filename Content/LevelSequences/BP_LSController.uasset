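; Level sequence controller that switches between sequences from a LevelSequences array, keeping the active player in ChosenSequence.
; Pressing K stops the current sequence, plays the second entry once, then after a fixed half-second delay replaces it with the third, looping indefinitely.
; The OptionsMenu event is empty, and logic to play the first entry once is present but disconnected.
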(event `Key|K`
  (params (Key :type "Key Structure"))
  (bind _chosen_sequence (`self.Chosen Sequence`))
  (bind _chosen_sequence_2 (`self.Chosen Sequence`))
  (:`Pressed`
    (`/Engine/EditorBlueprintResources/StandardMacros.IsValid` _chosen_sequence
      (:`Is Valid`
        (`MovieSceneSequencePlayer.Stop` _chosen_sequence))
      (:`Is Not Valid`
        _))
    (bind (_outactor _returnvalue) (`LevelSequencePlayer.CreateLevelSequencePlayer` (`|GetArrayItem` (`self.Level Sequences`) 1) (make `MovieSceneSequencePlaybackSettings` false (`self.Don't Loop`))))
    (bind _output_get (set `self.Chosen Sequence` _returnvalue))
    (`MovieSceneSequencePlayer.Play` _output_get)
    (`KismetSystemLibrary.Delay` 0.5)
    (`/Engine/EditorBlueprintResources/StandardMacros.IsValid` _chosen_sequence_2
      (:`Is Valid`
        (`MovieSceneSequencePlayer.Stop` _chosen_sequence_2))
      (:`Is Not Valid`
        _))
    (bind (_outactor_2 _returnvalue_2) (`LevelSequencePlayer.CreateLevelSequencePlayer` (`|GetArrayItem` (`self.Level Sequences`) 2) (make `MovieSceneSequencePlaybackSettings` false (`self.Loop Indefinitely`))))
    (bind _output_get_2 (set `self.Chosen Sequence` _returnvalue_2))
    (`MovieSceneSequencePlayer.Play` _output_get_2)))

(event `OptionsMenu`)

(fn `UserConstructionScript`)